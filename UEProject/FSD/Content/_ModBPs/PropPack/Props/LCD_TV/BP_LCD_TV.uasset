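; BP_LCD_TV is an LCD TV prop that plays media from a playlist under keyboard control.
; BeginPlay enables input from player controller 0, so the actor responds to key events directly.
; Hardcoded keys drive a MediaPlayer to open the playlist, toggle play and pause, and skip to the next or previous entry.
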(event Custom|BeginPlay
  (Input|EnableInput (Game|GetPlayerController 0)))

(event Input|KeyboardEvents|E
  (params (Key :type Key%20Structure :default "None"))
  ;[1 1 1] Next Song
  (:Pressed
    (Class|MediaPlayer|Next (Variables|Default|GetMedia%20Player))))

(event Input|KeyboardEvents|Q
  (params (Key :type Key%20Structure :default "None"))
  ;[1 1 1] Previous Song
  (:Pressed
    (Class|MediaPlayer|Previous (Variables|Default|GetMedia%20Player))))

(event Input|KeyboardEvents|F
  (params (Key :type Key%20Structure :default "None"))
  ;[1 1 1] Start Song's in the Playlist
  (:Pressed
    (Class|MediaPlayer|OpenPlaylist (Variables|Default|GetMedia%20Player) "/Game/_ModBPs/PropPack/Props/LCD_TV/MediaPlaylist.MediaPlaylist")))

(event Input|KeyboardEvents|G
  (params (Key :type Key%20Structure :default "None"))
  (bind _media_player (Variables|Default|GetMedia%20Player))
  ;[1 1 1] Play/Pause
  (:Pressed
    (if (Audio|Components|Audio|IsPlaying _media_player)
      (Sequencer|Player|Pause _media_player)
      (else
        (Media|MediaPlayer|Play _media_player :!class /Script/MediaAssets.MediaPlayer)))))

(fn ConstructionScript)